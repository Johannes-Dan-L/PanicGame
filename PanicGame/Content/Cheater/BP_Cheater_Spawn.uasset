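; Turret-style spawner that aims at nearby pawns and launches Cheater actors from its SpawnPoint socket.
; Each tick it picks the closest pawn within sensing range that has line of sight from the Spawner component.
; The Spawner turns toward that target at constant speed with clamped pitch, firing once the cooldown has passed and a dot-product check confirms it faces the target.
; A DoN gate, reset on each shot, caps the spawns per shot.
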(event `self.ReceiveTick`
  (params (DeltaSeconds :type "Float (single-precision)"))
  (`self.FindTarget`)
  (`self.Target`
    (:`then`
      (`self.UpdateSpawnerRotation` DeltaSeconds)
      (`self.UpdateFire`))
    (:`else`)))

(event `Fire`
  (set `self.TimeOfLastFire` (`KismetSystemLibrary.GetGameTimeInSeconds`))
  (`|ExecutionSequence`
    (:`then_0`
      (goto _label :!via `Reset`))
    (:`then_1`
      (`/Engine/EditorBlueprintResources/StandardMacros.Do N` 1 :!label _label
        (:`Exit`
          (`|SpawnActorFromClass` "/Game/Cheater/Cheater.Cheater_C" (`SceneComponent.GetSocketTransform` (`self.Spawner`) "SpawnPoint" "RTS_World") "Undefined" "OverrideRootScale" null null)
          (`KismetSystemLibrary.Delay` 0.2)
          (goto _label))))))

(fn `FindTarget`
  (locals (`CurrentDistance(Local)` :type "Float (double-precision)") (`BestDistance(Local)` :type "Float (double-precision)") (`BestTarget(Local)` :type "Actor Object Reference") (`CurrentTarget(Local)` :type "Actor Object Reference"))
  (set `local.BestDistance(Local)` (+ (`self.SensingRange`) 1.0))
  (bind _outactors (`KismetSystemLibrary.SphereOverlapActors` (`self.K2_GetActorLocation`) (`self.SensingRange`) (`|MakeArray` "ObjectTypeQuery3" :!type "EObjectTypeQuery Enum") "/Script/Engine.Actor"))
  (for _array_element _outactors
    (bind _output_get (set `local.CurrentTarget(Local)` _array_element))
    (bind _output_get_2 (set `local.CurrentDistance(Local)` (`self.GetDistanceTo` _output_get self)))
    (if (or (< _output_get_2 (`local.BestDistance(Local)`)) (not (`KismetSystemLibrary.IsValid` (`local.BestTarget(Local)`))))
      (bind _result (`/Game/Cheater/BPFunctionLibrary.HasLineOfSight` (`SceneComponent.K2_GetComponentLocation` (`self.Spawner`)) (`self.K2_GetActorLocation` (`local.CurrentTarget(Local)`)) (`|MakeArray` self (`local.CurrentTarget(Local)`) :!type "Actor Object Reference")))
      (if _result
        (set `local.BestTarget(Local)` (`local.CurrentTarget(Local)`))
        (set `local.BestDistance(Local)` (`local.CurrentDistance(Local)`)))))
  (set `self.Target` (`local.BestTarget(Local)`)))

(fn `UpdateFire`
  (if (> (- (`KismetSystemLibrary.GetGameTimeInSeconds`) (`self.TimeOfLastFire`)) (`self.RateOfFire`))
    (if (> (`KismetMathLibrary.Dot_VectorVector` (`KismetMathLibrary.GetDirectionUnitVector` (`SceneComponent.K2_GetComponentLocation` (`self.Spawner`)) (`self.K2_GetActorLocation` (`self.Target`))) (`SceneComponent.GetForwardVector` (`self.Spawner`))) 0.99)
      (`self.Fire`) ; If No Cooldown & It is facing the target then Fire
    )))

(fn `UpdateSpawnerRotation`
  (params (DeltaSeconds :type "Float (double-precision)"))
  (locals (NewRotation :type "Rotator Structure" :default (struct)))
  (bind _output_get (set `local.NewRotation` (`KismetMathLibrary.RInterpTo_Constant` (`SceneComponent.K2_GetComponentRotation` (`self.Spawner`)) (`KismetMathLibrary.FindLookAtRotation` (`SceneComponent.K2_GetComponentLocation` (`self.Spawner`)) (`self.K2_GetActorLocation` (`self.Target`))) (`local.DeltaSeconds`) (`self.RotationSpeed`))))
  (`SceneComponent.K2_SetWorldRotation` (`self.Spawner`) (`KismetMathLibrary.MakeRotator` (.roll _output_get) (`KismetMathLibrary.ClampAngle` (.pitch _output_get) -45.0 75.0) (.yaw _output_get)) false false))

(fn `UserConstructionScript`)