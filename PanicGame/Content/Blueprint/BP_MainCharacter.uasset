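; Main character Blueprint that turns captured audio loudness into movement of its Sphere component and removes Cheater actors on contact.
; Audio capture envelope values select one of three positions along local Y, with louder input sending the Sphere farther via timed MoveComponentTo.
; A box collider destroys any overlapping Cheater, while Tick only prints a debug message when the Bride's CheaterCheating flag is set.
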(event `self.AudioCapture.OnAudioEnvelopeValue`
  (params (EnvelopeValue :type "Float (single-precision)"))
  (bind _sphere (`self.Sphere`))
  ;[1 1 1] Movement
  (`KismetSystemLibrary.PrintString` (`KismetStringLibrary.Conv_DoubleToString` EnvelopeValue) false)
  (if (> EnvelopeValue 0.007)
    (if (> EnvelopeValue 0.02)
      (`KismetSystemLibrary.MoveComponentTo` _sphere (0.0 -680.0 0.0) (struct) false false 0.3)
      (`KismetSystemLibrary.PrintString` "further")
      (else
        (`KismetSystemLibrary.MoveComponentTo` _sphere (0.0 -330.0 0.0) (struct) true true 0.3)
        (`KismetSystemLibrary.PrintString` "mid")))
    (else
      (`KismetSystemLibrary.MoveComponentTo` _sphere (0.0 0.0 0.0) (struct) false false 0.3))))

(event `self.BoxCollider.OnComponentBeginOverlap`
  (params (OverlappedComponent :type "PrimitiveComponent Object Reference") (OtherActor :type "Actor Object Reference") (OtherComp :type "PrimitiveComponent Object Reference") (OtherBodyIndex :type Integer) (bFromSweep :type Boolean) (SweepResult :type "HitResult Structure (by ref)"))
  ;[1 1 1] Destroys the Cheaters when collided with player
  (bind _ascheater (cast `/Game/Cheater/Cheater` OtherActor))
  (`self.K2_DestroyActor` _ascheater))

(event `self.ReceiveTick`
  (params (DeltaSeconds :type "Float (single-precision)"))
  (if (`/Game/Bride/Bride_Pawn.CheaterCheating` (`self.Bride`))
    (`KismetSystemLibrary.PrintString` "cheat")))

(fn `UserConstructionScript`)